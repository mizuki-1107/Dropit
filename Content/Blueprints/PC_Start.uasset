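; PC_Start is the player controller for the start screen, handling the title UI and the jump into a random stage.
; BeginPlay enables mouse input, shows UI_Start with a fade-in, and passes it the saved high score from BP_Player after a zero-length delay.
; Event_OpenRandomStage plays a UI_Fade fade-out, then opens a zero-prefixed Map_Stage level picked at random from StageNumbers.
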(event `self.ReceiveBeginPlay`
  (`|ExecutionSequence`
    (:`then_0`
      ;[1 1 1] Player
      (`|ExecutionSequence`
        (:`then_0`
          (set `self.PlayerRef` (cast `/Game/Blueprints/BP_Player` (`self.K2_GetPawn`) :!pure true))
          ;;[1 1 1] Set Mouse Input
          (set `self.bShowMouseCursor` true)
          (`WidgetBlueprintLibrary.SetInputMode_GameAndUIEx` self null "DoNotLock" false))
        (:`then_1`
          (`KismetSystemLibrary.Delay` 0.0)
          (set `/Game/UI/UI_Start.HighScore` (`/Game/Blueprints/BP_Save.HighScore` (`/Game/Blueprints/BP_Player.SaveRef` (`self.PlayerRef`))) (`self.UI_Start`)))))
    (:`then_1`
      (`|ExecutionSequence`
        (:`then_0`
          ;[1 1 1] UI_Start
          (bind _returnvalue (`|CreateWidget` "/Game/UI/UI_Start.UI_Start_C" null self))
          (bind _output_get (set `self.UI_Start` _returnvalue))
          (`UserWidget.AddToPlayerScreen` _output_get 0)
          (`|PlayAnimation` _output_get (`/Game/UI/UI_Start.FadeIn` _returnvalue)))
        (:`then_1`
          ;[1 1 1] FadeIn
          (bind _returnvalue_2 (`|CreateWidget` "/Game/UI/UI_Fade.UI_Fade_C"))
          (`UserWidget.AddToViewport` _returnvalue_2 0)
          (`|PlayAnimation` _returnvalue_2 (`/Game/UI/UI_Fade.Fade` _returnvalue_2) 0.0 1 "Reverse"
            (:`Finished`
              (`Widget.RemoveFromParent` _returnvalue_2))))))))

(event `Event_OpenRandomStage`
  ;[1 1 1] Event_OpenRandomStage
  ;;[1 1 1] FadeOut
  (bind _returnvalue (`|CreateWidget` "/Game/UI/UI_Fade.UI_Fade_C"))
  (`UserWidget.AddToViewport` _returnvalue 0)
  (`|PlayAnimation` _returnvalue (`/Game/UI/UI_Fade.Fade` _returnvalue)
    (:`Finished`
      (bind _result (`BlueprintSetLibrary.Set_ToArray` (`self.stageNumbers`)))
      ;;[1 1 1] OpenRandomMap
      (`GameplayStatics.OpenLevel` (`KismetStringLibrary.Conv_StringToName` (`KismetStringLibrary.Concat_StrStr` "Map_Stage_" (`KismetStringLibrary.Concat_StrStr` "0" (`KismetStringLibrary.Conv_IntToString` (`|GetArrayItem` _result (`KismetMathLibrary.RandomInteger` (`KismetArrayLibrary.Array_Length` _result)))))))) ; ランダムなステージを開く
    )))

(fn `UserConstructionScript`)