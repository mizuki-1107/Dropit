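; Block tower actor that builds downward-stacked rings of spline-mesh segments, each with one tagged, differently colored breakable segment.
; GenerateStages runs in construction or at BeginPlay per IsGenerate, creating materials and sampling a temporary circular spline for segment positions and tangents.
; GenerateStage builds each ring under its own scene component, re-randomizing the breakable index at a set stage frequency.
; Helper functions check breakability, remove a segment's stage, and play break effects; BreakStage is empty.
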(event `self.ReceiveBeginPlay`
  (if (not (`self.IsGenerate?`))
    (`self.GenerateStages`)))

(event `GenerateStages`
  (bind _blockcount (`self.BlockCount`))
  (`|ExecutionSequence`
    (:`then_0`
      (`KismetArrayLibrary.Array_Clear` (`self.StageRoot`))
      (bind _returnvalue (`KismetMaterialLibrary.CreateDynamicMaterialInstance` "/Game/Materials/M_Ball_Inst.M_Ball_Inst"))
      (bind _output_get (set `self.M_BreakableBlock` _returnvalue))
      (`MaterialInstanceDynamic.SetVectorParameterValue` _output_get "Color" (`self.BreakableColor`))
      (bind _returnvalue_2 (`KismetMaterialLibrary.CreateDynamicMaterialInstance` "/Game/Materials/M_Ball_Inst.M_Ball_Inst"))
      (bind _output_get_2 (set `self.M_UnbreakableBlock` _returnvalue_2))
      (`MaterialInstanceDynamic.SetVectorParameterValue` _output_get_2 "Color" (`self.UnBreakableColor`)))
    (:`then_1`
      (`|ExecutionSequence`
        (:`then_0`
          (`KismetArrayLibrary.Array_Clear` (`self.Locations`))
          (`KismetArrayLibrary.Array_Clear` (`self.Tangents`))
          (bind _returnvalue_3 (`AddComponent|NODE_AddSplineComponent-0`))
          (set `self.Spline` _returnvalue_3)
          (`SplineComponent.ClearSplinePoints` _returnvalue_3 true)
          (for _index (range _blockcount)
            (`SplineComponent.AddSplinePoint` _returnvalue_3 (* (`KismetMathLibrary.GetForwardVector` (`KismetMathLibrary.MakeRotator` 0.0 0.0 (* (`KismetMathLibrary.Conv_IntToDouble` _index) (/ 360.0 (`KismetMathLibrary.Conv_IntToDouble` _blockcount))))) (`self.Radius`)) "Local" true)
            (`SplineComponent.UpdateSpline` _returnvalue_3))
          (for _index_2 (range (`self.BlockCount`))
            (bind (_location _tangent) (`SplineComponent.GetLocationAndTangentAtSplinePoint` (`self.Spline`) _index_2 "Local"))
            (`KismetArrayLibrary.Array_Add` (`self.Tangents`) _tangent)
            (`KismetArrayLibrary.Array_Add` (`self.Locations`) _location))
          (`ActorComponent.K2_DestroyComponent` (`self.Spline`)))
        (:`then_1`
          (for _ (range (`self.StageCount`))
            (`self.GenerateStage`)))))))

(fn `BreakStage`
  (params (ItemToFind :type "PrimitiveComponent Object Reference (by ref)")))

(fn `GenerateStage`
  (locals (BreakbleNum_l :type Integer))
  (bind _tangents (`self.Tangents`))
  (bind _locations (`self.Locations`))
  (bind _returnvalue (`KismetMathLibrary.MakeVector2D` (`self.Width`) (`self.Thickness`)))
  (bind _returnvalue_2 (`KismetMathLibrary.MakeVector` 0.0 0.0 (* (* (`KismetMathLibrary.Conv_IntToDouble` (`self.CurrentStageCount`)) (`self.StageDistance`)) -1.0)))
  (`|ExecutionSequence`
    (:`then_0`
      (`/Engine/EditorBlueprintResources/StandardMacros.IncrementInt` (`self.CurrentStageCount`)))
    (:`then_1`
      (if (== (mod (`self.CurrentStageCount`) (`self.ChangeBreakableFrequency`)) 0)
        (set `local.BreakbleNum_l` (`KismetMathLibrary.RandomInteger` (`self.BlockCount`)))
        (set `self.BreakableNum` (`local.BreakbleNum_l`))))
    (:`then_2`
      (bind _returnvalue_3 (`AddComponent|NODE_AddSceneComponent-0`))
      (`KismetArrayLibrary.Array_Add` (`self.StageRoot`) _returnvalue_3)
      (for _index (range (`self.BlockCount`))
        (`|ExecutionSequence`
          (:`then_0`
            (bind _returnvalue_4 (`AddComponent|NODE_AddSplineMeshComponent-0`))
            (bind _returnvalue_5 (mod (+ _index 1) (`self.BlockCount`)))
            (`SplineMeshComponent.SetStartAndEnd` _returnvalue_4 (+ (`|GetArrayItem` _locations _index) _returnvalue_2) (`|GetArrayItem` _tangents _index) (+ (`|GetArrayItem` _locations _returnvalue_5) _returnvalue_2) (`|GetArrayItem` _tangents _returnvalue_5) false)
            (bind _returnvalue_6 (== _index (`self.BreakableNum`)))
            (`PrimitiveComponent.SetMaterial` _returnvalue_4 0 (select `bool` _returnvalue_6 :`false` (`self.M_UnbreakableBlock`) :`true` (`self.M_BreakableBlock`) :!type "MaterialInterface Object Reference"))
            (`SceneComponent.K2_AttachToComponent` _returnvalue_4 _returnvalue_3 "None" "KeepRelative" "KeepRelative" "KeepRelative" true)
            (`SplineMeshComponent.SetStartScale` _returnvalue_4 _returnvalue false)
            (`SplineMeshComponent.SetEndScale` _returnvalue_4 _returnvalue false)
            (`SplineMeshComponent.UpdateMesh` _returnvalue_4))
          (:`then_1`
            (if _returnvalue_6
              (set `ActorComponent.ComponentTags` (`|MakeArray` (`KismetStringLibrary.Conv_StringToName` (`self.BreakableTag`))) _returnvalue_4))))))))

(fn `GetCanBreak?`
  (params (self2 :type "ActorComponent Object Reference"))
  (returns (ReturnValue :type Boolean))
  (return (`ActorComponent.ComponentHasTag` self2 (`KismetStringLibrary.Conv_StringToName` (`self.BreakableTag`)))))

(fn `PlayBreakSound`
  (params (Location :type "Vector Structure") (PitchMultiplier :type "Float (double-precision)"))
  (`GameplayStatics.PlaySoundAtLocation` "/Game/Sound/Break_Cue.Break_Cue" Location (struct) 1.0 PitchMultiplier 0.0 null null null null))

(fn `Remove Stage by Component`
  (params (ItemToFind :type "PrimitiveComponent Object Reference (by ref)"))
  (locals (Com :type "Array of SceneComponent Object Reference") (StageRoot_l :type "SceneComponent Object Reference"))
  (set `local.StageRoot_l` (`SceneComponent.GetAttachParent` ItemToFind))
  (bind _output_get (set `local.Com` (`SceneComponent.GetChildrenComponents` (`local.StageRoot_l`) false)))
  (for _array_element _output_get
    (`ActorComponent.K2_DestroyComponent` _array_element))
  (`KismetArrayLibrary.Array_RemoveItem` (`self.StageRoot`) (`local.StageRoot_l`)))

(fn `SpawnBreakParticle`
  (params (Location :type "Vector Structure"))
  (bind _returnvalue (`GameplayStatics.SpawnEmitterAtLocation` "/Game/Particles/P_Break.P_Break" Location))
  (`FXSystemComponent.SetColorParameter` _returnvalue "BreakableColor" (`self.BreakableColor`))
  (`FXSystemComponent.SetColorParameter` _returnvalue "UnBreakableColor" (`self.UnBreakableColor`)))

(fn `UserConstructionScript`
  (if (`self.IsGenerate?`)
    (`self.GenerateStages`)))