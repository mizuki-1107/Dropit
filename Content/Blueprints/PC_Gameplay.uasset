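; Gameplay player controller that sets up the gameplay UI, relays touch input to BP_Player and saves the high score.
; On BeginPlay it plays the fade animation in reverse, shows the cursor, caches the controlled pawn and hands it a new gameplay widget.
; Touch press, release and move events pass 2D position and finger index to the pawn.
; A save event writes the given high score to the save slot.
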(event `self.ReceiveBeginPlay`
  (`|ExecutionSequence`
    (:`then_0`
      ;[1 1 1] FadeIn
      (bind _returnvalue (`|CreateWidget` "/Game/UI/UI_Fade.UI_Fade_C"))
      (`UserWidget.AddToViewport` _returnvalue 0)
      (`|PlayAnimation` _returnvalue (`/Game/UI/UI_Fade.Fade` _returnvalue) 0.0 1 "Reverse"))
    (:`then_1`
      (set `self.PlayerRef` (cast `/Game/Blueprints/BP_Player` (`self.K2_GetPawn`) :!pure true))
      (set `PlayerController.bShowMouseCursor` true (`GameplayStatics.GetPlayerController` 0))
      ;[1 1 1] Gameplay
      (bind _returnvalue_2 (`|CreateWidget` "/Game/UI/UI_Gameplay.UI_Gameplay_C"))
      (bind _output_get (set `/Game/Blueprints/BP_Player.UI` _returnvalue_2 (`self.PlayerRef`)))
      (`UserWidget.AddToPlayerScreen` _output_get 0))))

(event `Event_SaveScore`
  (params (HighScore :type Integer))
  (bind _saveref (`self.SaveRef`))
  (set `/Game/Blueprints/BP_Save.HighScore` HighScore _saveref)
  (`GameplayStatics.SaveGameToSlot` _saveref (`self.SaveSlotName`)))

(event `InputTouch`
  (params (Location :type "Vector Structure") (FingerIndex :type "ETouchIndex Enum"))
  (bind _playerref (`self.PlayerRef`))
  (bind _returnvalue (`KismetMathLibrary.MakeVector2D` (.x Location) (.y Location)))
  (:`Pressed`
    (`/Game/Blueprints/BP_Player.Event_Pressed` _playerref _returnvalue FingerIndex))
  (:`Released`
    (`/Game/Blueprints/BP_Player.Event_Released` _playerref _returnvalue FingerIndex))
  (:`Moved`
    (`/Game/Blueprints/BP_Player.Event_Moved` _playerref _returnvalue FingerIndex)))

(fn `UserConstructionScript`)